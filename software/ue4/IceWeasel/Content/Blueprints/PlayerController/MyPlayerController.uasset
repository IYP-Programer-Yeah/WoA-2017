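; Player controller that manages the local player's pause menu, toggled scoreboard and team-colored multiplayer chat.
; Input actions toggle the widgets; pause and chat also switch input mode, and pause disables pawn input without pausing the game.
; ServerReplicateMessage relays chat through the game mode's controller array, coloring sender names by each receiver's team relation.
; Each receiving controller adds the message to its chat widget, playing a fade-out when chat is closed.
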(event Custom|Show%20Pause%20Menu
  ;[1 1 1] Show / Hide Pause Menu
  (UserInterface|Viewport|AddtoViewport (Variables|Reference|GetPauseMenuRef) 0)
  (Input|DisableInput (Game|Player|GetPlayerPawn 0) (Game|GetPlayerController 0))
  (Variables|Default|SetbShowMouseCursor true)
  (Input|SetInputModeGameandUI self 0 "DoNotLock" true)
  (Variables|Default|SetPauseMenuActive true))

(event Custom|Server%20Replicate%20Message
  (params (Sender :type Text) (Message :type Text) (Player%20Controller :type Player%20Controller%20Object%20Reference))
  ;[1 1 1] Chat system
  (Chat|ReplicateChatMessage Sender Message Player%20Controller))

(event Custom|Show%20Chat%20Window
  (bind _chatwindowref (Variables|Reference|GetChatWindowRef))
  (bind _chatwindowref_2 (Variables|Reference|GetChatWindowRef))
  ;[1 1 1] Show / Hide Chat WIndow
  (Widget|SetVisibility (Variables|/Game/Widgets/HUD/ChatWindow.ChatWindow_C|GetChatInputTextBox _chatwindowref) "Visible") ; Show Input text box
  (Class|Border|SetBrushColor (Variables|/Game/Widgets/HUD/ChatWindow.ChatWindow_C|GetMessageListBorder _chatwindowref) (Variables|Default|GetChatBorderBrushColor))
  (Widget|SetVisibility (Variables|/Game/Widgets/HUD/ChatWindow.ChatWindow_C|GetMessageList _chatwindowref) "Visible") ; Show the message list
  (Class|UserWidget|StopAnimation _chatwindowref_2 (Variables|/Game/Widgets/HUD/ChatWindow.ChatWindow_C|GetFadeOut _chatwindowref_2)) ; Stop the fadeout animation
  (Input|SetInputModeGameandUI self (Variables|/Game/Widgets/HUD/ChatWindow.ChatWindow_C|GetChatInputTextBox (Variables|Reference|GetChatWindowRef)) "DoNotLock" true)
  (Variables|Default|SetChatWindowActive true))

(event Custom|Add%20Chat%20Message%20On%20Client
  (params (Sender :type Text) (Message :type Text) (Sender%20Text%20Color :type Linear%20Color%20Structure) (Message%20Text%20Color :type Linear%20Color%20Structure))
  ;[1 1 1] Chat system
  (Chat|AddChatMessage Sender Message Sender%20Text%20Color Message%20Text%20Color))

(event Custom|Hide%20Pause%20Menu
  ;[1 1 1] Show / Hide Pause Menu
  (Widget|RemovefromParent (Variables|Reference|GetPauseMenuRef))
  (Input|EnableInput (Game|Player|GetPlayerPawn 0) (Game|GetPlayerController 0))
  (Variables|Default|SetbShowMouseCursor false)
  (Input|SetInputModeGameOnly self)
  (Variables|Default|SetPauseMenuActive false))

(event Custom|Hide%20Chat%20Window
  (bind _chatwindowref (Variables|Reference|GetChatWindowRef))
  (bind _chatwindowref_2 (Variables|Reference|GetChatWindowRef))
  ;[1 1 1] Show / Hide Chat WIndow
  (Widget|SetVisibility (Variables|/Game/Widgets/HUD/ChatWindow.ChatWindow_C|GetChatInputTextBox _chatwindowref) "Hidden") ; Hide Input text box
  (Class|Border|SetBrushColor (Variables|/Game/Widgets/HUD/ChatWindow.ChatWindow_C|GetMessageListBorder _chatwindowref) "(R=0.000000,G=0.000000,B=0.000000,A=0.000000)") ; Opacity = 0 (Invisible)
  (Widget|SetVisibility (Variables|/Game/Widgets/HUD/ChatWindow.ChatWindow_C|GetMessageList _chatwindowref) "Hidden") ; Hide the message list
  (Class|UserWidget|StopAnimation _chatwindowref_2 (Variables|/Game/Widgets/HUD/ChatWindow.ChatWindow_C|GetFadeOut _chatwindowref_2)) ; Stop the fadeout animation
  (Input|SetInputModeGameOnly self)
  (Variables|Default|SetChatWindowActive false))

(event EventBeginPlay
  (|CallParentFunction)
  (Utilities|FlowControl|Sequence
    (:then_0
      (Development|PrintString "Blueprint BeginPlay!" true true "(R=0.000000,G=0.660000,B=1.000000,A=1.000000)" 1e+01))
    (:then_1
      ;[1 1 1] Initialize Necessary things
      (if (Pawn|IsLocalPlayerController)
        (bind _returnvalue (UserInterface|CreateWidget "/Game/Widgets/HUD/ChatWindow.ChatWindow_C" self))
        (bind _output_get (Variables|Reference|SetChatWindowRef _returnvalue))
        (UserInterface|Viewport|AddtoViewport _output_get 0)
        (Class|Border|SetBrushColor (Variables|/Game/Widgets/HUD/ChatWindow.ChatWindow_C|GetMessageListBorder _output_get) "(R=0.000000,G=0.000000,B=0.000000,A=0.000000)") ; Opacity = 0 (Invisible)
        (Widget|SetVisibility (Variables|/Game/Widgets/HUD/ChatWindow.ChatWindow_C|GetChatInputTextBox _output_get) "Hidden")))))

(event Input|ActionEvents|InputActionPause
  (params (Key :type Key%20Structure :default "AnyKey"))
  ;[1 1 1] Show / Hide Pause Menu
  (:Pressed
    (Utilities|IsValid (Variables|Reference|GetPauseMenuRef)
      (:Is%20Valid
        _)
      (:Is%20Not%20Valid
        (bind _returnvalue (UserInterface|CreateWidget "/Game/Widgets/PauseMenu/PauseMenu.PauseMenu_C" (Game|GetPlayerController 0)))
        (Variables|Reference|SetPauseMenuRef _returnvalue)))
    (if (Variables|Default|GetPauseMenuActive)
      (CallFunction|HidePauseMenu)
      (else
        (CallFunction|ShowPauseMenu)))))

(event Input|ActionEvents|InputActionScoreboard
  (params (Key :type Key%20Structure :default "AnyKey"))
  ;[1 1 1] Show / Hide Scoreboard
  (:Pressed
    (Utilities|FlowControl|FlipFlop
      (:A
        (Utilities|IsValid (Variables|Reference|GetScoreboardRef)
          (:Is%20Valid
            _)
          (:Is%20Not%20Valid
            (bind _returnvalue (UserInterface|CreateWidget "/Game/Widgets/HUD/Scoreboard.Scoreboard_C" self))
            (Variables|Reference|SetScoreboardRef _returnvalue)))
        (Default|ClearScoreboardEntries (Variables|Reference|GetScoreboardRef))
        (Default|UpdateScoreboard (Variables|Reference|GetScoreboardRef))
        (Utilities|FlowControl|Sequence
          (:then_0
            (Default|SetTeamName (Variables|Reference|GetScoreboardRef) 0 "Team 0")
            (Default|SetTeamName (Variables|Reference|GetScoreboardRef) 1 "Team 1"))
          (:then_1
            (UserInterface|Viewport|AddtoViewport (Variables|Reference|GetScoreboardRef) 0))))
      (:B
        (Utilities|IsValid (Variables|Reference|GetScoreboardRef)
          (:Is%20Valid
            (Widget|RemovefromParent (Variables|Reference|GetScoreboardRef))))))))

(event Input|ActionEvents|InputActionChat
  (params (Key :type Key%20Structure :default "AnyKey"))
  ;[1 1 1] Show / Hide Chat WIndow
  (:Pressed
    (if (Variables|Default|GetChatWindowActive)
      (CallFunction|HideChatWindow)
      (else
        (CallFunction|ShowChatWindow)))))

(fn ConstructionScript)

(fn AddChatMessage
  (params (Sender :type Text) (Message :type Text) (Sender%20Text%20Color :type Linear%20Color%20Structure) (Message%20Text%20Color :type Linear%20Color%20Structure))
  (bind _chatwindowref (Variables|Reference|GetChatWindowRef))
  (bind _chatwindowref_2 (Variables|Reference|GetChatWindowRef))
  (Utilities|IsValid _chatwindowref
    (:Is%20Valid
      (if (Variables|Default|GetChatWindowActive)
        (Widget|SetVisibility (Variables|/Game/Widgets/HUD/ChatWindow.ChatWindow_C|GetMessageList _chatwindowref_2) "Visible") ; Don't play fadeout animation in case the chat window is already\nactive - just add the message to the window
        (else
          (UserInterface|Animation|PlayAnimation _chatwindowref_2 (Variables|/Game/Widgets/HUD/ChatWindow.ChatWindow_C|GetFadeOut _chatwindowref) 0.0 1 "Forward" 1.0) ; When a message is received,\nshow the message and play the fadeout animation\n\n(The animation handles showing of the message aswell)
        ))
      (Default|AddChatMessage (Variables|Reference|GetChatWindowRef) Sender Message Sender%20Text%20Color Message%20Text%20Color))))

(fn ReplicateChatMessage
  (params (Sender :type Text) (Message :type Text) (Player%20Controller :type Player%20Controller%20Object%20Reference))
  (Utilities|FlowControl|Sequence
    (:then_0
      (LocalVariables|SetSenderText Sender)
      (LocalVariables|SetMessageText Message))
    (:then_1
      (bind _asbase_game_mode (Utilities|Casting|CastToBaseGameMode (Game|GetGameMode)))
      (bind _asmy_player_state (Utilities|Casting|CastToMyPlayerState (Variables|/Script/Engine.Controller|GetPlayerState Player%20Controller)))
      (for _array_element (Variables|/Script/IceWeasel.BaseGameMode|GetPlayerControllerArray _asbase_game_mode) ; Add the message to the ChatWindow widget for every player that is\nsuccessfully connected
        (bind _asmy_player_controller (Utilities|Casting|CastToMyPlayerController _array_element))
        (bind _asmy_player_state_2 (Utilities|Casting|CastToMyPlayerState (Variables|/Script/Engine.Controller|GetPlayerState _array_element)))
        (if (== (Variables|/Script/IceWeasel.BasePlayerState|GetTeamNum _asmy_player_state_2) (Variables|/Script/IceWeasel.BasePlayerState|GetTeamNum _asmy_player_state)) ; Does this person who is receiving message has\nsame team as the one who is sending message?
          (CallFunction|AddChatMessageonClient _asmy_player_controller (LocalVariables|GetSenderText) (LocalVariables|GetMessageText) "(R=0.000000,G=1.000000,B=0.000000,A=1.000000)" "(R=1.000000,G=1.000000,B=1.000000,A=1.000000)") ; Green color for friendlies
          (elif (== (Variables|/Script/IceWeasel.BasePlayerState|GetTeamNum _asmy_player_state_2) -1)
            (CallFunction|AddChatMessageonClient _asmy_player_controller (LocalVariables|GetSenderText) (LocalVariables|GetMessageText) "(R=1.000000,G=1.000000,B=1.000000,A=1.000000)" "(R=1.000000,G=1.000000,B=1.000000,A=1.000000)") ; Red color for enemies
            (else
              (CallFunction|AddChatMessageonClient _asmy_player_controller (LocalVariables|GetSenderText) (LocalVariables|GetMessageText) "(R=1.000000,G=0.000000,B=0.000000,A=1.000000)" "(R=1.000000,G=1.000000,B=1.000000,A=1.000000)") ; Red color for enemies
            )))))))