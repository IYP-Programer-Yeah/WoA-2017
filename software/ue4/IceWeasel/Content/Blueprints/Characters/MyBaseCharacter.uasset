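; Base character Blueprint that shows the player's name and provides helpers for orienting the character to a normal.
; Tick copies the name from a valid PlayerState into the PlayerName text every frame.
; ComputeCharacterRotation builds a rotation with Z on the given normal and X toward the current forward.
; SmoothOutRotation interpolates the actor's rotation toward a target; neither helper is called here.
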(event EventBeginPlay)

(event EventTick
  (params (DeltaSeconds :type Float%20%28single-precision%29))
  (bind _playerstate (Variables|Default|GetPlayerState))
  (Utilities|FlowControl|Sequence
    (:then_0
      (Utilities|IsValid _playerstate
        (:Is%20Valid
          (Rendering|Components|TextRender|SetText (Variables|Default|GetPlayerName) (Utilities|Text|ToText(String) (Variables|/Script/Engine.PlayerState|GetPlayerName _playerstate))))))))

(fn ConstructionScript)

(fn ComputeCharacterRotation
  (params (Normal :type Vector))
  (return (Math|Rotator|MakeRotfromZX Normal (Math|Vector|GetForwardVector (Transformation|GetActorRotation)))))

(fn SmoothOutRotation
  (params (Input%20Rotation :type Rotator))
  (return (Math|Interpolation|RInterpTo (Transformation|GetActorRotation) Input%20Rotation (Utilities|Time|GetWorldDeltaSeconds) 15.0)))